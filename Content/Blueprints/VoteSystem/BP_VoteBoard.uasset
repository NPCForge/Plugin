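; Village vote board that stores who votes against whom and swaps its mesh depending on whether any votes are posted.
; ModifyVote replaces a voter's previous entry in VoteList, RemoveVote withdraws it and EraseBoardContent clears the board, each refreshing the mesh.
; GetVoteResults tallies targets in a map keyed by character enum, returning the most-voted villagers, a tie flag and vote totals.
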(event Custom|Erase%20Board%20Content
  (Utilities|Array|Clear (Variables|Default|GetVoteList))
  (CallFunction|UpdateBoardMesh))

(event Custom|Modify%20Vote
  (params (New%20vote :type S%20Villager%20Vote%20Structure))
  (Variables|Default|SetIncoming%20Vote New%20vote)
  (for (_array_element _array_index) (Variables|Default|GetVoteList)
    (if (Utilities|Enum|Equal(Enum) (.CharacterEnum (Utilities|Struct|BreakS_CharacterInfo (Utilities|Struct|BreakS_VillagerVote _array_element))) (.CharacterEnum (Utilities|Struct|BreakS_CharacterInfo (Utilities|Struct|BreakS_VillagerVote (Variables|Default|GetIncoming%20Vote)))))
      (Utilities|Array|RemoveIndex (Variables|Default|GetVoteList) _array_index)))
  (Utilities|Array|Add (Variables|Default|GetVoteList) (Variables|Default|GetIncoming%20Vote))
  (CallFunction|UpdateBoardMesh))

(event Custom|Update%20Board%20Mesh
  (Components|StaticMesh|SetStaticMesh (Variables|Default|GetSM_Board) (select (> (Utilities|Array|Length (Variables|Default|GetVoteList)) 0) "/Game/Fantastic_Village_Pack/meshes/props/deco/SM_PROP_board_01.SM_PROP_board_01" "/Game/Fantastic_Village_Pack/meshes/props/deco/SM_PROP_board_02.SM_PROP_board_02")))

(fn ConstructionScript)

(fn GetVoteResults
  (bind _mostvotedcharacters (Variables|Default|GetMostVotedCharacters))
  (bind _mostvotedcharacters_2 (Variables|Default|GetMostVotedCharacters))
  ;[0 0 0] Reads the "VoteList" variable and output a list with the most voted villager(s) in it.
  (for _array_element (Variables|Default|GetVoteList)
    (if (.ReturnValue (Utilities|Map|Find (Variables|Default|GetVoteCounts) (.CharacterEnum (Utilities|Struct|BreakS_CharacterInfo (Utilities|Struct|BreakS_VillagerVote _array_element)))))
      (Math|Integer|IncrementInt (.Value (Utilities|Map|Find (Variables|Default|GetVoteCounts) (.CharacterEnum (Utilities|Struct|BreakS_CharacterInfo (Utilities|Struct|BreakS_VillagerVote _array_element))))))
      (else
        (Utilities|Map|Add (Variables|Default|GetVoteCounts) (.CharacterEnum (Utilities|Struct|BreakS_CharacterInfo (Utilities|Struct|BreakS_VillagerVote _array_element))) 1))))
  (bind _enumvalue (|ForEachE_Character)
    (:LoopBody
      (if (.ReturnValue (Utilities|Map|Find (Variables|Default|GetVoteCounts) _enumvalue))
        (if (> (.Value (Utilities|Map|Find (Variables|Default|GetVoteCounts) _enumvalue)) (LocalVariables|GetI_BiggestVoteCount))
          (LocalVariables|SetI_BiggestVoteCount (.Value (Utilities|Map|Find (Variables|Default|GetVoteCounts) _enumvalue)))
          (Utilities|Array|Clear _mostvotedcharacters)
          (Utilities|Array|Add _mostvotedcharacters _enumvalue :!label _label)
          (elif (== (.Value (Utilities|Map|Find (Variables|Default|GetVoteCounts) _enumvalue)) (LocalVariables|GetI_BiggestVoteCount))
            (goto _label)))))
    (:then
      (return (Utilities|Array|IsNotEmpty _mostvotedcharacters_2) _mostvotedcharacters_2 (> (Utilities|Array|Length _mostvotedcharacters_2) 1) (LocalVariables|GetI_BiggestVoteCount) (Utilities|Array|Length (Variables|Default|GetVoteList))))))

(fn RemoveVote
  (params (Character :type S%20Character%20Info%20Structure))
  ;[0 0 0] Remove the vote of a specified character from the VoteList.
  (LocalVariables|SetDesisting%20Character Character)
  (for (_array_element _array_index) (Variables|Default|GetVoteList)
    (if (Utilities|Enum|Equal(Enum) (.CharacterEnum (Utilities|Struct|BreakS_CharacterInfo (Utilities|Struct|BreakS_VillagerVote _array_element))) (.CharacterEnum (Utilities|Struct|BreakS_CharacterInfo (LocalVariables|GetDesisting%20Character))))
      (Utilities|Array|RemoveIndex (Variables|Default|GetVoteList) _array_index)
      (LocalVariables|SetB_VoteFound true)))
  (CallFunction|UpdateBoardMesh)
  (return (LocalVariables|GetB_VoteFound)))
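; BP_AI is an NPC whose messages appear on its own chat display widget and in the player's chat recap.
; Construction looks up the character slot's DataTable row to store character info and set the skeletal mesh, printing an error if missing.
; NPCForge send-message events update the widget and forward the text with character info to the player's HUD handler.
; Debug text and AI move-to-player snippets remain unconnected.
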(event OnSendMessage(NPCForge)
  (params (Message :type String))
  (bind _returnvalue (Utilities|Text|ToText(String) Message))
  (Default|SetTextDisplay (Variables|Default|GetChat%20Display%20Widget) _returnvalue)
  (CallFunction|AddChattoRecap _returnvalue))

(event Custom|Add%20chat%20to%20Recap
  (params (Text :type Text))
  ;[1 1 1] Send chat to Player's Recap Widget
  (Default|AddChattoRecap (Variables|/Game/Blueprints/BP_Player_v2.BP_Player_v2_C|GetBPC_HUD_Handler (Variables|Default|GetPlayer%20Ref)) (Variables|Default|GetCharacter%20Infos) Text))

(event Custom|Debug%20Text
  (bind _debugtxt (Variables|Default|GetDebugTxt))
  (bind _debugtxt2 (Variables|Default|GetDebugTxt2))
  (bind _b_debug (Variables|Default|GetB_Debug))
  (bind _returnvalue (select _b_debug _debugtxt _debugtxt2))
  ;[1 1 1] Debug text display
  (Utilities|FlowControl|Delay (Variables|Default|GetF_DebugDelay))
  (Default|SetTextDisplay (Variables|Default|GetChat%20Display%20Widget) _returnvalue)
  (CallFunction|AddChattoRecap _returnvalue))

(event EventBeginPlay
  (bind _aswbp_chat_display (Utilities|Casting|CastToWBP_ChatDisplay (UserInterface|GetUserWidgetObject (Variables|Default|GetChatDisplayComponent))))
  (Variables|Default|SetChat%20Display%20Widget _aswbp_chat_display))

(fn ConstructionScript
  (bind _characterslot (Variables|Default|GetCharacterSlot))
  (bind _returnvalue (Utilities|GetDataTableRow (.datatable (.datarow _characterslot)) (.rowname (.datarow _characterslot)))
    (:then
      (bind _output_get (Variables|Default|SetCharacter%20Infos _returnvalue))
      (Components|SkeletalMesh|SetSkeletalMeshAsset (Variables|Character|GetMesh) (Utilities|Struct|BreakS_CharacterInfo _output_get)))
    (:RowNotFound
      (Development|PrintText (Utilities|Text|FormatText "ERROR: Character Slot data row not found with name \"{name}\"." (.rowname (.datarow _characterslot))) true true "(R=1.000000,G=0.000000,B=0.002383,A=1.000000)" 6e+02))))

(fn GetGameRole
  (return (Utilities|String|EnumtoString (Variables|Default|GetGameRole))))
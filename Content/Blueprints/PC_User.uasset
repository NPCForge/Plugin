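; PC_User is a player controller that gives the player a chat recap overlay and a key to advance the game phase.
; On BeginPlay it creates a hidden WBP_ChatRecap widget on the viewport and caches the GM_MyGameMode reference.
; T toggles the recap between visible and hidden, and N calls GoNextGamePhase on the game mode.
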(event Custom|Create%20Chat%20Recap%20Widget
  ;[0 1 0.008331] Chat Recap
  (bind _returnvalue (UserInterface|CreateWidget "/Game/Widgets/ChatRecap/WBP_ChatRecap.WBP_ChatRecap_C" self))
  (bind _output_get (Variables|Default|SetWBP%20Chat%20Recap _returnvalue))
  (UserInterface|Viewport|AddtoViewport _output_get 0)
  (Widget|SetVisibility _output_get "Hidden"))

(event EventBeginPlay
  (Utilities|FlowControl|Sequence
    (:then_0
      (CallFunction|CreateChatRecapWidget))
    (:then_1
      (bind _asgm_my_game_mode (Utilities|Casting|CastToGM_MyGameMode (Game|GetGameMode)))
      (Variables|Default|SetGamemode%20Ref _asgm_my_game_mode))))

(event Input|KeyboardEvents|T
  (params (Key :type Key%20Structure :default "None"))
  (bind _wbp_chat_recap (Variables|Default|GetWBP%20Chat%20Recap))
  ;[0 1 0.008331] Chat Recap
  ;;[0 0 0] Press T to toggle chat recap
  (:Pressed
    (switch Utilities|FlowControl|Switch|SwitchonESlateVisibility (Variables|/Script/UMG.Widget|GetVisibility _wbp_chat_recap)
      (:Visible
        (Variables|/Script/UMG.Widget|SetVisibility _wbp_chat_recap "Hidden" :!label _label))
      (:Collapsed
        (goto _label))
      (:Hidden
        (Variables|/Script/UMG.Widget|SetVisibility _wbp_chat_recap "Visible"))
      (:HitTestInvisible
        (goto _label))
      (:SelfHitTestInvisible
        (goto _label)))))

(event Input|KeyboardEvents|N
  (params (Key :type Key%20Structure :default "None"))
  (:Pressed
    (Default|GoNextGamePhase (Variables|Default|GetGamemode%20Ref))))

(fn ConstructionScript)
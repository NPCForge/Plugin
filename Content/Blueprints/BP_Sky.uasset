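; BP_Sky is a day/night sky actor that drives a sun and a moon directional light from a 24-hour clock.
; SetSkyTime sets a target hour, and Tick advances the current time forward, scaled by time dilation and wrapping at 24, until it nearly matches.
; UpdateSky converts the time to light pitch, keeping the moon opposite the sun.
; The construction script applies rotation, intensity and color, and holds the starting time.
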(event Custom|Set%20Sky%20Time
  (params (New%20Time :type Float%20%28double-precision%29))
  ;[0 0 0] Set sky time, locking the time at designated time.
  (Variables|Default|SetF_TimeTarget New%20Time))

(event Custom|Update%20Sky
  (bind _f_currenttime (Variables|Default|GetF_CurrentTime))
  (bind _returnvalue (/ _f_currenttime 24.0))
  (bind _returnvalue_2 (* _returnvalue 3.6e+02))
  (bind _returnvalue_3 (+ _returnvalue_2 9e+01))
  (Utilities|FlowControl|Sequence
    (:then_0
      ;[0 0 0] Sun Rotation
      (Transformation|SetRelativeRotation (Variables|Default|GetDirectionalLight_Sun) (Math|Rotator|MakeRotator 0.0 _returnvalue_3 0.0) false false))
    (:then_1
      ;[0 0 0] Moon Rotation, opposite to the sun
      (Transformation|SetRelativeRotation (Variables|Default|GetDirectionalLight_Moon) (Math|Rotator|MakeRotator 0.0 (+ _returnvalue_3 1.8e+02) 0.0) false false))))

(event EventTick
  (params (DeltaSeconds :type Float%20%28single-precision%29))
  ;[0 0 0] Set sky time, locking the time at designated time.
  (if (not (Math|Float|NearlyEqual(Float) (Variables|Default|GetF_CurrentTime) (Variables|Default|GetF_TimeTarget) 0.1))
    (bind _output_get (Variables|Default|SetF_CurrentTime (+ (/ DeltaSeconds (Variables|Default|GetF_TimeDilation)) (Variables|Default|GetF_CurrentTime))))
    (if (>= _output_get 24.0)
      (Variables|Default|SetF_CurrentTime 0.0))
    (CallFunction|UpdateSky)))

(fn ConstructionScript
  (bind _directionallight_sun (Variables|Default|GetDirectionalLight_Sun))
  (bind _directionallight_moon (Variables|Default|GetDirectionalLight_Moon))
  (CallFunction|UpdateSky)
  (Utilities|FlowControl|Sequence
    (:then_0
      ;[0 0 0] Time Target by default at Current Time, so the sky don't change at the start of the simulation.
      (Variables|Default|SetF_TimeTarget (Variables|Default|GetF_CurrentTime)))
    (:then_1
      (Rendering|Components|Light|SetIntensity _directionallight_sun (Variables|Default|GetSunlight%20Intensity))
      (Rendering|Components|Light|SetLightColor _directionallight_sun (Variables|Default|GetSunlight%20Color) true))
    (:then_2
      (Rendering|Components|Light|SetIntensity _directionallight_moon (Variables|Default|GetMoonlight%20Intensity))
      (Rendering|Components|Light|SetLightColor _directionallight_moon (Variables|Default|GetMoonlight%20Color) true))))
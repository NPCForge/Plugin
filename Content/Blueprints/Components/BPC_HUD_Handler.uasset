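; BPC_HUD_Handler is a component on BP_Player_v2 that manages the player's chat recap and reset-game HUD widgets.
; On BeginPlay it caches its owner and adds both widgets to the viewport, with the chat recap hidden.
; The IA_ToggleChatRecap input flips recap visibility, the mouse cursor and the Enhanced Input mapping context between default and menu.
; AddChatToRecap forwards character info and text to the recap widget.
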(event Custom|Toggle%20Chat%20Recap
  (bind _wbp_chat_recap (Variables|Default|GetWBP%20Chat%20Recap))
  ;[0 0 0] Chat Recap
  (if (Variables|Default|GetB_FocusOnGame?)
    (Variables|Default|SetB_FocusOnGame? false)
    (Variables|/Script/UMG.Widget|SetVisibility _wbp_chat_recap "Visible")
    (CallFunction|SetMenuMode true)
    (else
      (Variables|Default|SetB_FocusOnGame? true)
      (Variables|/Script/UMG.Widget|SetVisibility _wbp_chat_recap "Hidden")
      (CallFunction|SetMenuMode false))))

(event Custom|Add%20Chat%20To%20Recap
  (params (Character%20Infos :type S%20Character%20Info%20Structure) (Text :type Text))
  ;[0 0 0] Chat Recap
  (Default|AddChat (Variables|Default|GetWBP%20Chat%20Recap) Text Character%20Infos))

(event Custom|Set%20Menu%20Mode
  (params (Menu%20Mode :type Boolean))
  (bind _owner_ref (Variables|Default|GetOwner%20Ref))
  (bind _player_controller (Variables|/Game/BP_Player_v2.BP_Player_v2_C|GetPlayer%20Controller _owner_ref))
  (bind _returnvalue (PlayerController|LocalPlayerSubsystems|GetEnhancedInputLocalPlayerSubsystem _player_controller))
  (bind _output_get (Variables|/Script/Engine.PlayerController|SetbShowMouseCursor (Variables|/Game/BP_Player_v2.BP_Player_v2_C|GetPlayer%20Controller (Variables|Default|GetOwner%20Ref)) Menu%20Mode))
  (if _output_get
    (Input|RemoveMappingContext _returnvalue "/Game/StartContent/ThirdPerson/Input/IMC_Default.IMC_Default" "(bIgnoreAllPressedKeysUntilRelease=True,bForceImmediately=False,bNotifyUserSettings=False)")
    (Input|AddMappingContext _returnvalue "/Game/StartContent/ThirdPerson/Input/IMC_Menu.IMC_Menu" 0 "(bIgnoreAllPressedKeysUntilRelease=True,bForceImmediately=False,bNotifyUserSettings=False)")
    (else
      (Input|RemoveMappingContext _returnvalue "/Game/StartContent/ThirdPerson/Input/IMC_Menu.IMC_Menu" "(bIgnoreAllPressedKeysUntilRelease=True,bForceImmediately=False,bNotifyUserSettings=False)")
      (Input|AddMappingContext _returnvalue "/Game/StartContent/ThirdPerson/Input/IMC_Default.IMC_Default" 0 "(bIgnoreAllPressedKeysUntilRelease=True,bForceImmediately=False,bNotifyUserSettings=False)"))))

(event Custom|Create%20Reset%20Game%20Widget
  (bind _returnvalue (UserInterface|CreateWidget "/Game/Widgets/WBP_ResetGameHUD.WBP_ResetGameHUD_C" (Variables|/Game/BP_Player_v2.BP_Player_v2_C|GetPlayer%20Controller (Variables|Default|GetOwner%20Ref))))
  (UserInterface|Viewport|AddtoViewport _returnvalue 0))

(event Custom|Create%20Chat%20Recap%20Widget
  ;[0 0 0] Chat Recap
  (bind _returnvalue (UserInterface|CreateWidget "/Game/Widgets/ChatRecap/WBP_ChatRecap.WBP_ChatRecap_C"))
  (bind _output_get (Variables|Default|SetWBP%20Chat%20Recap _returnvalue))
  (UserInterface|Viewport|AddtoViewport _output_get 0)
  (Widget|SetVisibility _output_get "Hidden"))

(event Input|EnhancedActionEvents|EnhancedInputActionIA_ToggleChatRecap
  (params (ActionValue :type Boolean) (ElapsedSeconds :type Float%20%28double-precision%29) (TriggeredSeconds :type Float%20%28double-precision%29) (InputAction :type Input%20Action%20Object%20Reference :default "/Game/StartContent/ThirdPerson/Input/Actions/IA_ToggleChatRecap.IA_ToggleChatRecap"))
  ;[0 0 0] Chat Recap
  (CallFunction|ToggleChatRecap))

(event EventBeginPlay
  (bind _asbp_player_v_2 (Utilities|Casting|CastToBP_Player_v2 (Components|GetOwner)))
  (Variables|Default|SetOwner%20Ref _asbp_player_v_2)
  (CallFunction|CreateChatRecapWidget)
  (CallFunction|CreateResetGameWidget))
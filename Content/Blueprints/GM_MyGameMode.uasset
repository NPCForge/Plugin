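; Game mode that randomly deals game roles to the NPC AIs on the map at level start.
; After a short delay, it checks that the BP_AI count matches the RoleMap total, then gives each AI a random role key, decrementing that key's remaining count.
; It prints a role recap or a mismatch error.
; It also stores the game phase and looks up character info in DT_Characters by enum name.
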(event Custom|Set%20Game%20Phase
  (params (GamePhase :type E_GamePhase%20Enum :default "NewEnumerator0"))
  (Variables|Default|SetGamePhase GamePhase))

(event EventBeginPlay
  (bind _rolemap (Variables|Default|GetRoleMap))
  (Utilities|FlowControl|Delay 1.0)
  (Utilities|FlowControl|Sequence
    (:then_0
      ;[0 0 0] Get required number of characters based on Role Map.
      (Variables|Default|SetI_CharactersNumber 0)
      (bind _values (Utilities|Map|Values (Variables|Default|GetRoleMap)))
      (for _array_element _values
        (Variables|Default|SetI_CharactersNumber (+ _array_element (Variables|Default|GetI_CharactersNumber)))))
    (:then_1
      ;[0 0 0] Get all AIs on the map.
      (bind _outactors (Actor|GetAllActorsOfClass "/Game/Blueprints/BP_AI.BP_AI_C"))
      (bind _output_get (Variables|Default|SetAI%20Actors _outactors))
      ;[0 0 0] Compare AIs number to Role Map.
      (if (== (Utilities|Array|Length _output_get) (Variables|Default|GetI_CharactersNumber))
        ;[0 0 0] Set AI Game Role by selecting a random key of Role Map.
        ; The Key value is decremented by one, if the value is below 1, it is removed from Role Map
        (for _array_element_2 (Variables|Default|GetAI%20Actors)
          (bind _keys (Utilities|Map|Keys _rolemap))
          (bind _output_get_2 (Variables|Default|SetRoleBuffer (.OutItem (Utilities|Array|Random _keys))))
          (bind _output_get_3 (Variables|/Game/Blueprints/BP_AI.BP_AI_C|SetGameRole _array_element_2 _output_get_2))
          (Variables|Default|SetI_ValueBuffer (.Value (Utilities|Map|Find _rolemap _output_get_2)))
          (Utilities|Map|Remove (Variables|Default|GetRoleMap) _output_get_3)
          (if (> (Variables|Default|GetI_ValueBuffer) 1)
            (Utilities|Map|Add (Variables|Default|GetRoleMap) _output_get_3 (- (Variables|Default|GetI_ValueBuffer) 1))))
        ;;[0.2365 0.2365 0.2365] Debug
        (Development|PrintString "-------ROLES RECAP------")
        (for _array_element_3 (Variables|Default|GetAI%20Actors)
          (Development|PrintText (Utilities|Text|FormatText "NPC {name} is a {role}" (Utilities|Struct|BreakS_CharacterInfo (Variables|/Game/Blueprints/BP_AI.BP_AI_C|GetCharacter%20Infos _array_element_3)) (Utilities|String|EnumtoString (Variables|/Game/Blueprints/BP_AI.BP_AI_C|GetGameRole _array_element_3))) true true "(R=0.000000,G=0.660000,B=1.000000,A=1.000000)" 6e+02))
        (Development|PrintString "-----------------------")
        (else
          (Development|PrintText (Utilities|Text|FormatText "ERROR: AIs number on map ({IAs nb}) does not match RoleMap's required number ({Role nb})." (Utilities|Array|Length _output_get) (Variables|Default|GetI_CharactersNumber)) true true "(R=1.000000,G=0.000000,B=0.002383,A=1.000000)" 6e+02))))))

(fn ConstructionScript)

(fn GetCharacterfromEnum
  (params (Character%20enum :type E_Character%20Enum :default "NewEnumerator0"))
  (bind _returnvalue (Utilities|String|EnumtoString Character%20enum))
  (bind _returnvalue_2 (Utilities|String|StringToName _returnvalue))
  (bind _returnvalue_3 (Utilities|GetDataTableRow "/Game/Characters/DT_Characters.DT_Characters" _returnvalue_2)
    (:then
      (return true _returnvalue_3))
    (:RowNotFound
      (Development|PrintText (Utilities|Text|FormatText "ERROR: Enum Character \"{enum}\" not found in Characters DataTable." _returnvalue_2))
      (return false ""))))
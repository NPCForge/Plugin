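; AI-driven NPC character that shows its chat messages on a widget component and logs them to the player's chat recap.
; The construction script pulls name, icon, color and skeletal mesh from the character's data table row.
; Messages from NPCForge update the display and go to the player's HUD handler with that identity.
; BeginPlay caches the widget and posts debug text after a short delay; a debug move-to-player node is unconnected.
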(event OnSendMessage(NPCForge)
  (params (Message :type String))
  (bind _returnvalue (Utilities|Text|ToText(String) Message))
  (Default|SetTextDisplay (Variables|Default|GetChat%20Display%20Widget) _returnvalue)
  (CallFunction|AddChattoRecap _returnvalue))

(event Custom|Add%20chat%20to%20Recap
  (params (Text :type Text))
  ;[1 1 1] Send chat to Player's Recap Widget
  (Default|AddChattoRecap (Variables|/Game/BP_Player_v2.BP_Player_v2_C|GetBPC_HUD_Handler (Variables|Default|GetPlayer%20Ref)) Text (Variables|Default|GetColor) (Variables|Default|GetCharacter%20Icon) (Variables|Default|GetCharacter%20Name)))

(event EventBeginPlay
  (bind _debugtxt (Variables|Default|GetDebugTxt))
  (bind _aswbp_chat_display (Utilities|Casting|CastToWBP_ChatDisplay (UserInterface|GetUserWidgetObject (Variables|Default|GetChatDisplayComponent))))
  (Variables|Default|SetChat%20Display%20Widget _aswbp_chat_display)
  ;[1 1 1] Debug text display
  (Utilities|FlowControl|Delay 0.1)
  (Default|SetTextDisplay (Variables|Default|GetChat%20Display%20Widget) _debugtxt)
  (CallFunction|AddChattoRecap _debugtxt))

(fn ConstructionScript
  (bind _characterinfos (Variables|Default|GetCharacterInfos))
  (bind _returnvalue (Utilities|GetDataTableRow (.datatable (.datarow _characterinfos)) (.rowname (.datarow _characterinfos)))
    (:then
      (Variables|Default|SetCharacter%20Name (.Name (Utilities|Struct|BreakS_CharacterInfo _returnvalue)))
      (Variables|Default|SetCharacter%20Icon (.Icon (Utilities|Struct|BreakS_CharacterInfo _returnvalue)))
      (Variables|Default|SetColor (.Color (Utilities|Struct|BreakS_CharacterInfo _returnvalue)))
      (Components|SkeletalMesh|SetSkeletalMeshAsset (Variables|Character|GetMesh) (.SkeletalMesh (Utilities|Struct|BreakS_CharacterInfo _returnvalue))))))